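; BP_CardController is a player controller for the card game UI and board pointing.
; On BeginPlay it creates the W_CardHud widget, adds it to the viewport, sets UI-only input focused on it and shows the cursor.
; GetMousePositionOnBoard deprojects the mouse into the world and moves along that ray by the view target's height minus a fixed offset, approximating a board point without a trace or plane intersection.
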(event EventBeginPlay
  (bind _returnvalue (UserInterface|CreateWidget "/Game/CardUI/W_CardHud.W_CardHud_C" self))
  (UserInterface|Viewport|AddtoViewport _returnvalue 0)
  (Input|SetInputModeUIOnly self _returnvalue "DoNotLock" false)
  (Variables|Default|SetbShowMouseCursor true))

(event EventTick
  (params (DeltaSeconds :type Float%20%28single-precision%29)))

(fn ConstructionScript)

(fn GetMousePositiononBoard
  (bind _self self)
  (bind (_locationx _locationy) (Game|Player|GetMousePosition _self))
  (bind (_worldlocation _worlddirection) (Class|PlayerController|DeprojectScreenPositiontoWorld _locationx _locationy))
  (return (+ _worldlocation (* _worlddirection (- (.Z (Math|Vector|BreakVector (Transformation|GetActorLocation (Pawn|GetViewTarget self)))) 1e+02)))))