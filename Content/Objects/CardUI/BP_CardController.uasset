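; Player controller for the card game that sets up the local player's card HUD and mouse-driven input.
; On BeginPlay it creates W_CardHud, switches to UI-only input and shows the cursor.
; An event switches the view target to a given camera.
; GetMousePositionOnBoard deprojects the cursor and steps along the ray by the view target's height minus a fixed offset, approximating a board point without a trace.
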(event Custom|AssignControllerToCameraView
  (params (TargetCamera :type Camera%20Actor%20Object%20Reference))
  (Game|Player|SetViewTargetwithBlend TargetCamera 0.0 "VTBlend_Linear" 0.0 false))

(event EventBeginPlay
  (bind _self self)
  (if (Pawn|IsLocalPlayerController _self)
    (bind _returnvalue (UserInterface|CreateWidget "/Game/Objects/CardUI/W_CardHud.W_CardHud_C" _self))
    (UserInterface|Viewport|AddtoViewport _returnvalue 0)
    (Input|SetInputModeUIOnly self _returnvalue "DoNotLock" false)
    (Variables|Default|SetbShowMouseCursor true)))

(fn ConstructionScript)

(fn GetMousePositiononBoard
  (bind _self self)
  (bind (_locationx _locationy) (Game|Player|GetMousePosition _self))
  (bind (_worldlocation _worlddirection) (Class|PlayerController|DeprojectScreenPositiontoWorld _locationx _locationy))
  (return (+ _worldlocation (* _worlddirection (- (.Z (Math|Vector|BreakVector (Transformation|GetActorLocation (Pawn|GetViewTarget self)))) 1e+02)))))