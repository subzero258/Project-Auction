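; Game mode for a two-player card game that connects players to level cameras, spawns the table actors and starts the match.
; BeginPlay spawns objective zones; joining players attach to cameras through a level interface after a short delay.
; When the second connects, it spawns three decks and fills them by suit from DT_Cards, with Clubs and Diamonds sharing one.
; Round start calls DealCardsToPlayers, which is still empty.
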(event Custom|BeginRound
  (params (RoundNumber :type Integer))
  (CallFunction|DealCardstoPlayers))

(event Custom|BeginGame
  (Development|PrintString "Begin Game")
  (CallFunction|CreateDecks)
  (CallFunction|DealStartingDecks)
  (CallFunction|BeginRound 1))

(event EventBeginPlay
  (CallFunction|CreateObjectiveZones))

(event EventHandleStartingNewPlayer
  (params (NewPlayer :type Player%20Controller%20Object%20Reference))
  (Utilities|FlowControl|Delay 0.5)
  (CallFunction|ConnectPlayertoCamera (Variables|/Script/Engine.Controller|GetPlayerState NewPlayer) (CallFunction|GetCurrentLevel))
  (bind _result (Math|Integer|IncrementInt (Variables|Default|GetNumberOfPlayersConnected))
    (:%20%20
      (if (== _result 2)
        (CallFunction|BeginGame)))))

(fn ConstructionScript)

(fn GetCurrentLevel
  (bind _outactors (Actor|GetAllActorswithInterface "/Game/Objects/Master/BPI_GameModeToLevel.BPI_GameModeToLevel_C"))
  (return (Utilities|Array|Get(acopy) _outactors)))

(fn ConnectAllCurrentPlayerstoCameras
  (for _array_element (Variables|/Script/Engine.GameStateBase|GetPlayerArray (Game|GetGameState))
    (Development|PrintString "Connecting Existing Player")
    (CallFunction|ConnectPlayertoCamera _array_element (CallFunction|GetCurrentLevel))))

(fn ConnectPlayertoCamera
  (params (PlayerState :type Player%20State%20Object%20Reference) (CurrentLevel :type Actor%20Object%20Reference))
  (bind _returnvalue (Utilities|Array|AddUnique (Variables|Default|GetConnectedPlayerStateList) PlayerState))
  (Class|BPIGameModetoLevel|AttachPlayertoCamera(Message) CurrentLevel (Game|GetPlayerController PlayerState) _returnvalue))

(fn CreateObjectiveZones
  (for _index (range 0 2)
    (bind _returnvalue (Game|SpawnActorfromClass "/Game/Objects/Board/BP_ObjectiveZone.BP_ObjectiveZone_C" (Utilities|Array|Get(acopy) (Variables|Default|GetCONST_ObjectiveSpawnLocations) _index) "Undefined" "MultiplyWithRoot" 0 0))
    (Utilities|Array|AddUnique (Variables|Default|GetObjectiveZones) _returnvalue)))

(fn CreateDecks
  (for _index (range 0 2)
    (bind _returnvalue (Game|SpawnActorfromClass "/Game/Objects/Board/BP_3DDeck.BP_3DDeck_C" (Utilities|Array|Get(acopy) (Variables|Default|GetCONST_DeckSpawnLocations) _index) "Undefined" "MultiplyWithRoot" 0 0))
    (Utilities|Array|AddUnique (Variables|Default|GetDeckReferences) _returnvalue)))

(fn DealStartingDecks
  (bind _outrownames (DataTable|GetDataTableRowNames "/Game/Objects/CardUI/DT_Cards.DT_Cards"))
  (for _array_element _outrownames
    (bind _returnvalue (Utilities|GetDataTableRow "/Game/Objects/CardUI/DT_Cards.DT_Cards" _array_element)
      (:then
        (switch string (.CardSuit (Utilities|Struct|BreakS_CardInfo _returnvalue))
          (:Spades
            (Class|BPIAddCard|AddCard(Message) (Utilities|Array|Get(acopy) (Variables|Default|GetDeckReferences) 1) _returnvalue))
          (:Hearts
            (Class|BPIAddCard|AddCard(Message) (Utilities|Array|Get(acopy) (Variables|Default|GetDeckReferences) 2) _returnvalue))
          (:Clubs
            (Class|BPIAddCard|AddCard(Message) (Utilities|Array|Get(acopy) (Variables|Default|GetDeckReferences)) _returnvalue :!label _label))
          (:Diamonds
            (goto _label)))))))

(fn DealCardstoPlayers)